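; BP_Boss1 is a boss enemy with a two-stage fight.
; On first perceiving the player it turns aggro, shows a health bar widget and unpauses boss music.
; HealthComponent damage spawns numbers and drives timeline knockback; at half health the boss teleports to Stage2Location, pauses and breaks the floor.
; Death removes the bar and starts music-box audio; other events handle knockback abilities, charge hits and a target arrow.
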(event `self.ReceiveBeginPlay`
  (bind _returnvalue (`GameplayStatics.SpawnSound2D` "/Game/Audio/Sounds/Enemies/236814__thejack288__music-box-lullaby.236814__thejack288__music-box-lullaby" 1.0 1.0 0.0 null))
  (bind _output_get (set `self.Musicbox` _returnvalue))
  (`AudioComponent.SetPaused` _output_get true)
  (bind _returnvalue_2 (`GameplayStatics.SpawnSound2D` "/Game/Audio/Sounds/BossMusic.BossMusic" 1.0 1.0 0.0 null))
  (bind _output_get_2 (set `self.BossAudio` _returnvalue_2))
  (`AudioComponent.SetPaused` _output_get_2 true)
  (bind _aswbp_healthbar (cast `/Game/Blueprints/UI/WBP_Healthbar` (`WidgetComponent.GetUserWidgetObject` (`self.Cast Bar`))))
  (bind _output_get_3 (set `self.As WBP Healthbar` _aswbp_healthbar))
  (set `/Game/Blueprints/UI/WBP_Healthbar.Health` (`HealthComponent.GetCurrentHealth` (`self.HealthComponent`)) _output_get_3)
  (set `/Game/Blueprints/UI/WBP_Healthbar.MaxHealth` (`HealthData.MaxHealth` (`HealthComponent.HealthSettings` (`self.HealthComponent`))) _output_get_3)
  (set `self.WalkSpeed` (`CharacterMovementComponent.MaxWalkSpeed` (`self.CharacterMovement`)))
  (message `/Game/Blueprints/Interfaces/BPI_CastbarBOss.Castbarget` (`WidgetComponent.GetUserWidgetObject` (`self.Cast Bar`)) self false))

(event `self.AIPerception.OnPerceptionUpdated`
  (params (UpdatedActors :type "Array of Actor Object Reference (by ref)"))
  ;[1 0.3408 0.4006] Aggro when player is seen
  (for _array_element UpdatedActors
    (if (== _array_element (`GameplayStatics.GetPlayerCharacter` 0))
      (`/Engine/EditorBlueprintResources/StandardMacros.DoOnce` false
        (:`Completed`
          (bind _asenemy_aicontroller (cast `EnemyAIController` (`self.GetController`)))
          (`EnemyAIController.BecomeAggro` _asenemy_aicontroller)
          (bind _returnvalue (`|CreateWidget` "/Game/Blueprints/UI/WB_BossHP.WB_BossHP_C"))
          (set `self.BossHp` _returnvalue)
          (`UserWidget.AddToViewport` _returnvalue 0)
          (`AudioComponent.SetPaused` (`self.BossAudio`) false))))))

(event `self.HealthComponent.OnDamage`
  (params (Amount :type Integer))
  (bind (_returnvalue_location _returnvalue_rotation) (`KismetMathLibrary.BreakTransform` (`self.GetTransform` (`self.Stage 2 Location`))))
  (bind _ratio (`self.Health to ratio`))
  (`/Game/Blueprints/UI/WB_BossHP.Update Health` (`self.BossHp`) _ratio)
  (`self.SpawnDmgNumbers` Amount)
  (if (`self.Knockback`)
    (`self.KnockbackFunc`))
  (if (<= _ratio 0.5)
    (`/Engine/EditorBlueprintResources/StandardMacros.DoOnce` false
      (:`Completed`
        (`self.K2_SetActorLocationAndRotation` _returnvalue_location _returnvalue_rotation false true)
        (`self.PauseBoss` 6.0)
        (`/Game/Blueprints/Level/BP_BrokenFloor.Break Floor` (`self.Floor`))))))

(event `TpBack`
  (bind (_returnvalue_location _returnvalue_rotation) (`KismetMathLibrary.BreakTransform` (`self.GetTransform` (`self.Stage 2 Location`))))
  (`self.K2_SetActorLocationAndRotation` _returnvalue_location _returnvalue_rotation false true))

(event `self.HealthComponent.OnDeath`
  (`Widget.RemoveFromParent` (`self.BossHp`))
  (`AudioComponent.SetPaused` (`self.BossMusic`) true)
  (`AudioComponent.SetPaused` (`self.Musicbox`) false))

(event `self.KnockbackFunc`
  (bind _locationbeforeknockback (`self.LocationBeforeKnockback`))
  ;[0.3467 1 0.1812 1 40] Knockback
  (`KismetSystemLibrary.PrintString` "Hello")
  (set `self.PlayerForwardBeforeKnockback` (`self.GetActorForwardVector` (`GameplayStatics.GetPlayerCharacter` 0)))
  (set `self.LocationBeforeKnockback` (`self.K2_GetActorLocation`))
  (bind (_direction _knockback_lerp) (`Timeline|Timeline` :!via `PlayFromStart`)
    (:`Update`
      (bind _sweephitresult (`self.K2_SetActorLocation` (`KismetMathLibrary.VLerp` _locationbeforeknockback (+ _locationbeforeknockback (* (`self.PlayerForwardBeforeKnockback`) 20.0)) _knockback_lerp) true))
      (bind (_bblockinghit _binitialoverlap _time _distance _location _impactpoint _normal _impactnormal _physmat _hitactor) (`GameplayStatics.BreakHitResult` _sweephitresult))
      (if _bblockinghit
        (message `/Game/Blueprints/Interfaces/BPI_Knockback.KnockbackFunc` _hitactor)))))

(event `/Game/Blueprints/Interfaces/BPI_KnockbackAbility.KnockbackAbility`
  (params (Location :type "Vector Structure") (Knockback :type "Float (double-precision)"))
  (bind _locationbeforeknockback (`self.LocationBeforeKnockback`))
  (bind _returnvalue (- (`self.LocationBeforeKnockback`) Location))
  ;[0.3467 1 0.1812 1 40] KnockbackAbility
  (set `self.Knockback` false)
  (`HealthComponent.Damage` (`self.HealthComponent`) 50)
  (set `self.LocationBeforeKnockback` (`self.K2_GetActorLocation`))
  (`/Engine/EditorBlueprintResources/StandardMacros.IsValid` self
    (:`Is Valid`
      (bind (_direction _alpha) (`Timeline|Timeline_0` :!via `PlayFromStart`)
        (:`Update`
          (`self.K2_SetActorLocation` (`KismetMathLibrary.VLerp` _locationbeforeknockback (+ _locationbeforeknockback (* (`KismetMathLibrary.Normal` _returnvalue) (- Knockback (`KismetMathLibrary.VSize` _returnvalue)))) _alpha) true))
        (:`Finished`
          (set `self.Knockback` true))))))

(event `/Game/Blueprints/Interfaces/BPI_GetArrow.SetArrow`
  (params (Visible :type Boolean))
  (bind _arrow1 (`self.Arrow1`))
  ;[1 1 1 1 30] Target Arrow
  (if Visible
    (`SceneComponent.SetVisibility` _arrow1 true false)
    (else
      (`SceneComponent.SetVisibility` _arrow1 false false))))

(event `/Game/Blueprints/Interfaces/BPI_Charge.Charge`
  (params (Damage :type "Float (double-precision)") (Knockback :type Boolean))
  ;[1 1 1 1 30] Charge
  (set `self.Knockback` Knockback)
  (`HealthComponent.Damage` (`self.HealthComponent`) (`KismetMathLibrary.FTrunc` Damage))
  (set `self.Knockback` true))

(fn `Health to ratio`
  (returns (Ratio :type "Float (double-precision)"))
  (bind _healthcomponent (`self.HealthComponent`))
  (return (/ (`KismetMathLibrary.Conv_IntToDouble` (`HealthComponent.GetCurrentHealth` _healthcomponent)) (`KismetMathLibrary.Conv_IntToDouble` (`HealthData.MaxHealth` (`HealthComponent.HealthSettings` _healthcomponent))))))

(fn `SpawnDmgNumbers`
  (params (Dmg :type Integer))
  (bind (_returnvalue_x _returnvalue_y) (`KismetMathLibrary.BreakVector` (`self.K2_GetActorLocation`)))
  (`|SpawnActorFromClass` "/Game/Blueprints/UI/BP_DamageNumbersActor.BP_DamageNumbersActor_C" (`KismetMathLibrary.MakeTransform` (`KismetMathLibrary.MakeVector` (+ _returnvalue_x 0.0) (+ _returnvalue_y (`KismetMathLibrary.RandomFloatInRange` -70.0 70.0)) 150.0)) "Undefined" "MultiplyWithRoot" null Dmg null))

(fn `UserConstructionScript`)