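; BP_HatredGrunt is a Hatred enemy that turns aggro through its AI controller when it first perceives the player.
; Damage from its HealthComponent updates the health bar, spawns damage numbers and flashes a hit overlay on body and mask.
; Swept timeline lerps drive knockback, which passes on to blocking actors, and a radial ability knockback followed by recovering walk speed.
; It also handles stuns, blocks, charge hits and a target arrow.
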(event `self.ReceiveBeginPlay`
  (bind _aswbp_healthbar (cast `/Game/Blueprints/UI/WBP_Healthbar` (`WidgetComponent.GetUserWidgetObject` (`self.HealthBar`))))
  (bind _output_get (set `self.As WBP Healthbar` _aswbp_healthbar))
  (set `/Game/Blueprints/UI/WBP_Healthbar.Health` (`HealthComponent.GetCurrentHealth` (`self.HealthComponent`)) _output_get)
  (set `/Game/Blueprints/UI/WBP_Healthbar.MaxHealth` (`HealthData.MaxHealth` (`HealthComponent.HealthSettings` (`self.HealthComponent`))) _output_get)
  (set `self.WalkSpeed` (`CharacterMovementComponent.MaxWalkSpeed` (`self.CharacterMovement`)))
  (message `/Game/Blueprints/Interfaces/BPI_castbar.Castbarget` (`WidgetComponent.GetUserWidgetObject` (`self.CastBar`)) self true))

(event `self.AIPerception.OnPerceptionUpdated`
  (params (UpdatedActors :type "Array of Actor Object Reference (by ref)"))
  ;[1 0.3408 0.4006] Aggro when player is seen
  (for _array_element UpdatedActors
    (if (== _array_element (`GameplayStatics.GetPlayerCharacter` 0))
      (`/Engine/EditorBlueprintResources/StandardMacros.DoOnce` false
        (:`Completed`
          (bind _asenemy_aicontroller (cast `EnemyAIController` (`self.GetController`)))
          (`EnemyAIController.BecomeAggro` _asenemy_aicontroller))))))

(event `self.HealthComponent.OnDamage`
  (params (Amount :type Integer))
  ;[1 1 1 1 40] On Damaged
  (`self.Spawn dmg numbers` Amount)
  (`self.SetOverlayMaterial` "/Game/LiamFolder/M_HitOVerlay_Inst.M_HitOVerlay_Inst")
  (set `/Game/Blueprints/UI/WBP_Healthbar.Health` (`HealthComponent.GetCurrentHealth` (`self.HealthComponent`)) (`self.As WBP Healthbar`))
  (if (`self.Knockback`)
    (`/Game/Blueprints/Interfaces/BPI_Knockback.KnockbackFunc`)
    (`SceneComponent.SetVisibility` (`self.HealthBar`) true false)
    (`KismetSystemLibrary.PrintString` (`KismetStringLibrary.Conv_IntToString` Amount))
    (else
      (`SceneComponent.SetVisibility` (`self.HealthBar`) true false)
      (`KismetSystemLibrary.Delay` 0.1)
      (`self.SetOverlayMaterial` null))))

(event `StunAction`
  (params (Duration :type "Float (double-precision)"))
  ;[0 1 1 1 30] Stun
  (`CharacterMovementComponent.DisableMovement` (`self.CharacterMovement`))
  (set `self.Stunned` true)
  (`KismetSystemLibrary.Delay` Duration)
  (set `self.Stunned` true)
  (`CharacterMovementComponent.SetMovementMode` (`self.CharacterMovement`) "MOVE_Walking" 0))

(event `/Game/Blueprints/Interfaces/BPI_Knockback.KnockbackFunc`
  (bind _locationbeforeknockback (`self.LocationBeforeKnockback`))
  ;[0.3467 1 0.1812 1 40] Knockback
  (set `self.PlayerForwardBeforeKnockback` (`self.GetActorForwardVector` (`GameplayStatics.GetPlayerCharacter` 0)))
  (set `self.LocationBeforeKnockback` (`self.K2_GetActorLocation`))
  (bind (_direction _knockback_lerp) (`Timeline|Timeline` :!via `PlayFromStart`)
    (:`Update`
      (bind _sweephitresult (`self.K2_SetActorLocation` (`KismetMathLibrary.VLerp` _locationbeforeknockback (+ _locationbeforeknockback (* (`self.PlayerForwardBeforeKnockback`) 100.0)) _knockback_lerp) true))
      (bind (_bblockinghit _binitialoverlap _time _distance _location _impactpoint _normal _impactnormal _physmat _hitactor) (`GameplayStatics.BreakHitResult` _sweephitresult))
      (if _bblockinghit
        (message `/Game/Blueprints/Interfaces/BPI_Knockback.KnockbackFunc` _hitactor)))
    (:`Finished`
      (`self.SetOverlayMaterial` null))))

(event `/Game/Blueprints/Interfaces/BPI_KnockbackAbility.KnockbackAbility`
  (params (Location :type "Vector Structure") (Knockback :type "Float (double-precision)"))
  (bind _locationbeforeknockback (`self.LocationBeforeKnockback`))
  (bind _returnvalue (- (`self.LocationBeforeKnockback`) Location))
  ;[0.3467 1 0.1812 1 40] KnockbackAbility
  (set `self.Knockback` false)
  (`HealthComponent.Damage` (`self.HealthComponent`) 50)
  (set `self.LocationBeforeKnockback` (`self.K2_GetActorLocation`))
  (`/Engine/EditorBlueprintResources/StandardMacros.IsValid` self
    (:`Is Valid`
      (bind (_direction _alpha) (`Timeline|Knockbacked` :!via `PlayFromStart`)
        (:`Update`
          (`self.K2_SetActorLocation` (`KismetMathLibrary.VLerp` _locationbeforeknockback (+ _locationbeforeknockback (* (`KismetMathLibrary.Normal` _returnvalue) (- Knockback (`KismetMathLibrary.VSize` _returnvalue)))) _alpha) true)
          (`self.DecaySlow`))
        (:`Finished`
          (set `self.Knockback` true))))))

(event `DecaySlow`
  ;[0.3467 1 0.1812 1 40] DecaySlow
  (bind (_direction _newtrack_0) (`Timeline|DecaySlowTimeline` :!via `PlayFromStart`)
    (:`Update`
      (set `CharacterMovementComponent.MaxWalkSpeed` (`KismetMathLibrary.Lerp` 0.0 (`self.WalkSpeed`) _newtrack_0) (`self.CharacterMovement`)))))

(event `/Game/Blueprints/Interfaces/BPI_GetArrow.SetArrow`
  (params (Visible :type Boolean))
  (bind _arrow1 (`self.Arrow1`))
  ;[1 1 1 1 30] Target Arrow
  (if Visible
    (`SceneComponent.SetVisibility` _arrow1 true false)
    (else
      (`SceneComponent.SetVisibility` _arrow1 false false))))

(event `/Game/Blueprints/Interfaces/BPI_Blocked.Blocked`
  (params (Duration :type "Float (double-precision)"))
  (`self.Stun` 2.0)
  (`self.SetOverlayMaterial` "/Game/LiamFolder/M_Stun.M_Stun")
  (`KismetSystemLibrary.Delay` 2.0)
  (`self.SetOverlayMaterial` null))

(event `/Game/Blueprints/Interfaces/BPI_Charge.Charge`
  (params (Damage :type "Float (double-precision)") (Knockback :type Boolean))
  ;[1 1 1 1 30] Charge
  (set `self.Knockback` Knockback)
  (`HealthComponent.Damage` (`self.HealthComponent`) (`KismetMathLibrary.FTrunc` Damage))
  (set `self.Knockback` true))

(fn `Spawn dmg numbers`
  (params (Dmg :type Integer))
  (bind (_returnvalue_x _returnvalue_y) (`KismetMathLibrary.BreakVector` (`self.K2_GetActorLocation`)))
  (`|SpawnActorFromClass` "/Game/Blueprints/UI/BP_DamageNumbersActor.BP_DamageNumbersActor_C" (`KismetMathLibrary.MakeTransform` (`KismetMathLibrary.MakeVector` (+ _returnvalue_x 0.0) (+ _returnvalue_y (`KismetMathLibrary.RandomFloatInRange` -70.0 70.0)) 160.0)) "Undefined" "MultiplyWithRoot" null Dmg null))

(fn `UserConstructionScript`)