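; BP_HudMessageTrigger is a level trigger that shows a configurable HUD message the first time the player pawn overlaps it.
; A DoOnce gate keeps it one-shot, and the player character's TextDisplayed flag decides whether to reuse the stored MsgHud widget or create one.
; A new WB_MSG_HUD receives the message and visible time, then is stored on the player; reuse only updates text and visibility.
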(event `self.Trigger.OnComponentBeginOverlap`
  (params (OverlappedComponent :type "PrimitiveComponent Object Reference") (OtherActor :type "Actor Object Reference") (OtherComp :type "PrimitiveComponent Object Reference") (OtherBodyIndex :type Integer) (bFromSweep :type Boolean) (SweepResult :type "HitResult Structure (by ref)"))
  (bind _as_player_character_bp (`self.As Player Character BP`))
  (bind _msghud (`/Game/Blueprints/Player/PlayerCharacter_BP.MsgHud` (`self.As Player Character BP`)))
  ;[1 1 1] Check if the actor that entered is the player
  (if (== OtherActor (`GameplayStatics.GetPlayerPawn` 0))
    (bind _asplayer_character_bp (cast `/Game/Blueprints/Player/PlayerCharacter_BP` (`GameplayStatics.GetPlayerCharacter` 0)))
    (set `self.As Player Character BP` _asplayer_character_bp)
    (`/Engine/EditorBlueprintResources/StandardMacros.DoOnce` false
      (:`Completed`
        (if (`/Game/Blueprints/Player/PlayerCharacter_BP.TextDisplayed` (`self.As Player Character BP`))
          (set `TextBlock.Text` (`KismetSystemLibrary.MakeLiteralText` (`self.HubMessage`)) (`/Game/Blueprints/UI/WB_MSG_HUD.Text` _msghud))
          (`Widget.SetVisibility` _msghud "Visible")
          (else
            (bind _returnvalue (`|CreateWidget` "/Game/Blueprints/UI/WB_MSG_HUD.WB_MSG_HUD_C" (`GameplayStatics.GetPlayerController` 0) (`KismetSystemLibrary.MakeLiteralText` (`self.HubMessage`)) (`self.Visible Time`)))
            (bind _output_get (set `self.Widget` _returnvalue))
            (`UserWidget.AddToViewport` _output_get 0)
            (set `/Game/Blueprints/Player/PlayerCharacter_BP.TextDisplayed` true _as_player_character_bp)
            (set `/Game/Blueprints/Player/PlayerCharacter_BP.MsgHud` _output_get _as_player_character_bp)))))))

(fn `UserConstructionScript`)