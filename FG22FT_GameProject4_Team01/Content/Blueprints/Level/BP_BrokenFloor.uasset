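; BP_BrokenFloor is a level actor that stages a floor collapse when BreakFloor is called.
; It resets the player camera to Default mode, shakes it, plays anticipation and laugh sounds, and reveals a set of NSFloorBreak effects.
; After a delay it plays an explosion sound, removes the effects and Box, and enables physics on the GeometryCollection.
; The actor destroys itself shortly afterwards.
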(event `Break Floor`
  (bind _returnvalue (`GameplayStatics.GetPlayerCharacter` 0))
  (bind _asplayer_character_bp (cast `/Game/Blueprints/Player/PlayerCharacter_BP` _returnvalue))
  (`GP4CharacterCameraComponent.SetCurrentCameraMode` (`GP4Character.GP4CharacterCamera` _asplayer_character_bp) "Default")
  (`GameplayStatics.PlayWorldCameraShake` "/Game/Blueprints/Player/CameraShake/BP_GroundCameraShake.BP_GroundCameraShake_C" (`self.K2_GetActorLocation` _returnvalue) 0.0 1000.0)
  (`GameplayStatics.PlaySound2D` "/Game/Audio/Sounds/Enemies/AnticipationFloordmg.AnticipationFloordmg" 1.0 1.0 0.0 null null)
  (`GameplayStatics.PlaySound2D` "/Game/Audio/Sounds/Enemies/Laugh.Laugh" 1.0 1.0 0.0 null null)
  (`SceneComponent.SetHiddenInGame` (`self.NS_FloorBreak1`) false false)
  (`SceneComponent.SetHiddenInGame` (`self.NS_FloorBreak`) false false)
  (`SceneComponent.SetHiddenInGame` (`self.NS_FloorBreak2`) false false)
  (`SceneComponent.SetHiddenInGame` (`self.NS_FloorBreak3`) false false)
  (`SceneComponent.SetHiddenInGame` (`self.NS_FloorBreak4`) false false)
  (`SceneComponent.SetHiddenInGame` (`self.NS_FloorBreak5`) false false)
  (`SceneComponent.SetHiddenInGame` (`self.NS_FloorBreak6`) false false)
  (`SceneComponent.SetHiddenInGame` (`self.NS_FloorBreak7`) false false)
  (`SceneComponent.SetHiddenInGame` (`self.NS_FloorBreak8`) false false)
  (`KismetSystemLibrary.Delay` 4.0)
  (`GameplayStatics.PlaySound2D` "/Game/Audio/Sounds/explfloor.explfloor" 1.0 1.0 0.0 null null)
  (`ActorComponent.K2_DestroyComponent` (`self.NS_FloorBreak`))
  (`ActorComponent.K2_DestroyComponent` (`self.NS_FloorBreak1`))
  (`ActorComponent.K2_DestroyComponent` (`self.NS_FloorBreak2`))
  (`ActorComponent.K2_DestroyComponent` (`self.NS_FloorBreak3`))
  (`ActorComponent.K2_DestroyComponent` (`self.NS_FloorBreak4`))
  (`ActorComponent.K2_DestroyComponent` (`self.NS_FloorBreak5`))
  (`ActorComponent.K2_DestroyComponent` (`self.NS_FloorBreak6`))
  (`ActorComponent.K2_DestroyComponent` (`self.NS_FloorBreak7`))
  (`ActorComponent.K2_DestroyComponent` (`self.NS_FloorBreak8`))
  (`ActorComponent.K2_DestroyComponent` (`self.Box`))
  (`PrimitiveComponent.SetSimulatePhysics` (`self.GeometryCollection`) true)
  (`KismetSystemLibrary.Delay` 2.0)
  (`self.K2_DestroyActor`))

(fn `UserConstructionScript`)