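; BP_TriggerLevel is a box trigger that moves the player to another level, optionally gated by and updating life stage progress.
; When the player pawn overlaps, it parses its Options string for a required stage and a stage to set in the ProgressSubsystem, with -1 meaning unset.
; If the gate passes, it plays a level sequence, waits briefly, opens the target level and destroys itself.
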(event `self.Box.OnComponentBeginOverlap`
  (params (OverlappedComponent :type "PrimitiveComponent Object Reference") (OtherActor :type "Actor Object Reference") (OtherComp :type "PrimitiveComponent Object Reference") (OtherBodyIndex :type Integer) (bFromSweep :type Boolean) (SweepResult :type "HitResult Structure (by ref)"))
  (bind _returnvalue (subsystem `ProgressSubsystem`))
  (bind _returnvalue_2 (`KismetStringLibrary.Concat_StrStr` "?" (`self.Options`)))
  (bind _returnvalue_3 (`GameplayStatics.GetIntOption` _returnvalue_2 "LifeStage" -1))
  (bind _returnvalue_4 (`GameplayStatics.GetIntOption` _returnvalue_2 "RequireLifeStage" -1))
  ;[1 1 1] Check if the actor that entered is the player
  (if (== OtherActor (`GameplayStatics.GetPlayerPawn` 0))
    (if (not (not (or (== (`ProgressSubsystem.GetLifeStageProgress` _returnvalue) _returnvalue_4) (== _returnvalue_4 -1))))
      (if (!= _returnvalue_3 -1)
        (`ProgressSubsystem.SetLifeStageProgress` _returnvalue _returnvalue_3))
      (bind (_outactor _returnvalue_5) (`LevelSequencePlayer.CreateLevelSequencePlayer` "/Game/Blueprints/MainLvlSequence.MainLvlSequence"))
      (`MovieSceneSequencePlayer.Play` _returnvalue_5)
      (`KismetSystemLibrary.Delay` 3.0)
      (`GameplayStatics.OpenLevelBySoftObjectPtr` (`self.Level`))
      (`self.K2_DestroyActor`))))

(fn `UserConstructionScript`)